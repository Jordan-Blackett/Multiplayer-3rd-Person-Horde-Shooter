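; Game mode for a horde game that scores bot kills and spawns AI bots.
; On each actor-killed event, it adds a fixed score to the killer's HordePlayerState when the victim is a non-player pawn, printing the total.
; SpawnNewBot runs an EQS query picking randomly from the best 25% of locations, then spawns BP_AICharacter at the returned points with debug spheres.
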(event Custom|OnActorKilled_Event_0
  (params (VictimActor :type Actor%20Object%20Reference) (KillerActor :type Actor%20Object%20Reference) (KillerController :type Controller%20Object%20Reference))
  (bind _aspawn (Utilities|Casting|CastToPawn VictimActor))
  (if (not (Pawn|IsPlayerControlled _aspawn))
    (bind _ashorde_player_state (Utilities|Casting|CastToHordePlayerState (Variables|/Script/Engine.Pawn|GetPlayerState (Pawn|GetControlledPawn KillerController))))
    (Class|HordePlayerState|AddScore _ashorde_player_state 1e+01)
    (Development|PrintString (Utilities|String|ToString(Float) (Variables|/Script/Engine.PlayerState|GetScore _ashorde_player_state)))))

(event Custom|OnQueryFinishedEvent_Event_0
  (params (QueryInstance :type Env%20Query%20Instance%20Blueprint%20Wrapper%20Object%20Reference) (QueryStatus :type EEnvQueryStatus%20Enum :default "Processing"))
  (switch Utilities|FlowControl|Switch|SwitchonEEnvQueryStatus QueryStatus
    (:Success
      (for _array_element (Class|EnvQueryInstanceBlueprintWrapper|GetResultsasLocations QueryInstance)
        (Rendering|Debug|DrawDebugSphere _array_element 5e+01 12 "(R=1.000000,G=0.935816,B=0.000000,A=1.000000)" 2.0 2.0)
        (Game|SpawnActorfromClass "/Game/Blueprints/AI/BP_AICharacter.BP_AICharacter_C" (Math|Transform|MakeTransform _array_element) "AdjustIfPossibleButDontSpawnIfColliding" 0 0)))))

(event EventBeginPlay
  (EventDispatchers|BindEventtoOnActorKilled (delegate Custom|OnActorKilled_Event_0)))

(event EventTick
  (params (DeltaSeconds :type Float%20%28single-precision%29)))

(event EventSpawnNewBot
  (bind _returnvalue (AI|EQS|RunEQSQuery "/Game/Blueprints/EQS_FindSpawnLocation.EQS_FindSpawnLocation" self "RandomBest25Pct"))
  (EventDispatchers|BindEventtoOnQueryFinishedEvent _returnvalue (delegate Custom|OnQueryFinishedEvent_Event_0)))

(fn ConstructionScript)