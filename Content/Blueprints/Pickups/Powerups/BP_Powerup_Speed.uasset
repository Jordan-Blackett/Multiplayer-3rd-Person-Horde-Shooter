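; Speed powerup pickup that temporarily doubles the movement speed of the actor that activated it.
; OnActivated sets MaxWalkSpeed on the owner's CharacterMovementComponent to twice GetMaxSpeed, and OnExpired sets it to half before calling the parent's expiry.
; Both read the live max speed, which varies with movement mode, rather than caching the original walk speed.
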(event EventBeginPlay)

(event Collision|EventActorBeginOverlap
  (params (OtherActor :type Actor%20Object%20Reference)))

(event EventTick
  (params (DeltaSeconds :type Float%20%28single-precision%29)))

(event EventOnExpired
  (bind _returnvalue (Class|HordePowerupActor|GetActivateOwner))
  (Variables|/Script/Engine.CharacterMovementComponent|SetMaxWalkSpeed (Actor|GetComponentbyClass _returnvalue "/Script/Engine.CharacterMovementComponent") (/ (Class|MovementComponent|GetMaxSpeed (Actor|GetComponentbyClass _returnvalue "/Script/Engine.CharacterMovementComponent")) 2.0))
  (|CallParentFunction))

(event EventOnActivated
  (bind _returnvalue (Class|HordePowerupActor|GetActivateOwner))
  (Variables|/Script/Engine.CharacterMovementComponent|SetMaxWalkSpeed (Actor|GetComponentbyClass _returnvalue "/Script/Engine.CharacterMovementComponent") (* (Class|MovementComponent|GetMaxSpeed (Actor|GetComponentbyClass _returnvalue "/Script/Engine.CharacterMovementComponent")) 2.0)))

(fn ConstructionScript)