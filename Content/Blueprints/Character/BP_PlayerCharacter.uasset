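; Player character Blueprint that sets up on-screen UI for the locally controlled player.
; On BeginPlay it adds a health indicator widget and a HUD widget to the viewport.
; Tick prints the health component's current value on screen as a debug readout, also only when locally controlled.
; Leftover unconnected nodes, including a rifle spawn and attach to the mesh's weapon socket, never run.
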(event EventBeginPlay
  (if (Pawn|IsLocallyControlled)
    (Utilities|FlowControl|Sequence
      (:then_1
        (bind _returnvalue (UserInterface|CreateWidget "/Game/UI/WBP_HealthIndicator.WBP_HealthIndicator_C"))
        (UserInterface|Viewport|AddtoViewport _returnvalue 0))
      (:then_2
        (bind _returnvalue_2 (UserInterface|CreateWidget "/Game/Blueprints/WidgetBP/HUD/WB_HUD_Widget.WB_HUD_Widget_C"))
        (UserInterface|Viewport|AddtoViewport _returnvalue_2 0)))))

(event Collision|EventActorBeginOverlap
  (params (OtherActor :type Actor%20Object%20Reference)))

(event EventTick
  (params (DeltaSeconds :type Float%20%28single-precision%29))
  (if (Pawn|IsLocallyControlled)
    (Development|PrintString (Utilities|String|ToString(Float) (Variables|/Script/HordeMode.HordeHealthComponent|GetHealth (Variables|Default|GetHealthComp))) true true "(R=0.000000,G=0.660000,B=1.000000,A=1.000000)" 0.0)))

(fn ConstructionScript)