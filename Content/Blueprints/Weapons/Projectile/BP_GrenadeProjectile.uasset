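; Grenade projectile that explodes on a short timed fuse after spawning, regardless of contact.
; BeginPlay waits out a delay, then calls Explode, which spawns a particle effect and applies full radial damage without falloff, credited to its instigator's controller.
; The actor then destroys itself and draws a brief debug sphere showing the damage radius.
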(event Custom|Explode
  (bind _returnvalue (Transformation|GetActorLocation))
  (Effects|SpawnEmitteratLocation "/Game/WeaponEffects/Explosion/P_Explosion.P_Explosion" _returnvalue)
  (Game|Damage|ApplyRadialDamage 1e+02 _returnvalue (Variables|Default|GetDamageRadius) 0 0 self (Game|GetInstigatorController) true "ECC_Visibility")
  (Actor|DestroyActor)
  (Rendering|Debug|DrawDebugSphere _returnvalue (Variables|Default|GetDamageRadius) 12 "(R=0.988370,G=1.000000,B=0.000000,A=1.000000)" 1.0 1.0))

(event EventBeginPlay
  (Utilities|FlowControl|Delay 1.0)
  (CallFunction|Explode))

(event Collision|EventActorBeginOverlap
  (params (OtherActor :type Actor%20Object%20Reference)))

(event EventTick
  (params (DeltaSeconds :type Float%20%28single-precision%29)))

(fn ConstructionScript)